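; Interactable button, the third "El" button by name, that toggles an electro on/off state and reports to a FinalButton.
; Focus toggles custom depth rendering on its mesh.
; Picking it while focused plays or reverses a timeline, depending on ElectroON, to slide the mesh slightly along Z.
; When the timeline finishes, it flips ElectroON and calls ThreeMessage on FinalButton.
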(event EventInterfaceToggleFocus
  (params (Focus :type Boolean))
  (Rendering|SetRenderCustomDepth (Variables|Default|GetStaticMesh) Focus))

(event EventInteractPick
  (if (stale EventInterfaceToggleFocus Focus)
    (if (Variables|Default|GetElectroON)
      (bind _screw_track (Timeline|Timeline Play)
        (:Update
          (Transformation|SetRelativeLocation (Variables|Default|GetStaticMesh) (Math|Vector|MakeVector 0.0 0.0 (Math|Float|Lerp 0.0 -2.0 _screw_track)) false false))
        (:Finished
          (if (Variables|Default|GetElectroON)
            (Variables|Default|SetElectroON false)
            (else
              (Variables|Default|SetElectroON true)))
          (Class|BIInteractThree|Three(Message) (Variables|Default|GetFinalButton))))
      (else
        (Timeline|Timeline Reverse)))))

(fn ConstructionScript)