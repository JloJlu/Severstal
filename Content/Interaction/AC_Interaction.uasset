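; Interaction component that detects the BP_InteractionArea the player is looking at and toggles its focus.
; Each tick it line-traces on Visibility from the player camera along its forward vector.
; When the hit actor changes or the trace misses, TraceInteractionArea updates the focused area; only the exact class matches, not subclasses.
; TryToInteract reads the focused area's Duration but does nothing with it yet.
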(event Custom|TryToInteract
  (params (In :type Boolean))
  (if In
    (if (Variables|Default|GetIsTracingInteractionArea)
      (bind _output_get (Variables|Default|SetDuration (Variables|/Game/Interaction/BP_InteractionArea.BP_InteractionArea_C|GetDuration (Variables|Default|GetFocusInteractionArea))))
      (if (> _output_get 0.0)
        _))))

(event EventTick
  (params (DeltaSeconds :type Float%20%28single-precision%29))
  (CallFunction|Trace))

(fn Trace
  (bind _returnvalue (Game|GetPlayerCameraManager 0))
  (bind _returnvalue_2 (Transformation|GetActorLocation _returnvalue))
  (bind (_outhit _returnvalue_3) (Collision|LineTraceByChannel _returnvalue_2 (+ _returnvalue_2 (* (Math|Vector|GetForwardVector (Transformation|GetActorRotation _returnvalue)) (Variables|Default|GetLenght))) "TraceTypeQuery1" false 0 "None"))
  (if _returnvalue_3
    (if (!= (Variables|Default|GetActor) (.HitActor (Collision|BreakHitResult _outhit)))
      (Variables|Default|SetActor (.HitActor (Collision|BreakHitResult _outhit)))
      (CallFunction|TraceInteractionArea (== (Utilities|GetClass (.HitActor (Collision|BreakHitResult _outhit))) "/Game/Interaction/BP_InteractionArea.BP_InteractionArea_C")))
    (else
      (CallFunction|TraceInteractionArea false))))

(fn TraceInteractionArea
  (params (Trace :type Boolean))
  (if Trace
    (if (Variables|Default|GetIsTracingInteractionArea)
      (Default|ToggleFocus (Variables|Default|GetFocusInteractionArea) false))
    (bind _asbp_interaction_area (Utilities|Casting|CastToBP_InteractionArea (Variables|Default|GetActor)))
    (bind _output_get (Variables|Default|SetFocusInteractionArea _asbp_interaction_area))
    (Default|ToggleFocus _output_get true)
    (Variables|Default|SetIsTracingInteractionArea true)
    (elif (Variables|Default|GetIsTracingInteractionArea)
      (Variables|Default|SetIsTracingInteractionArea false)
      (Default|ToggleFocus (Variables|Default|GetFocusInteractionArea) false)
      (Variables|Default|SetActor 0)
      (Variables|Default|SetFocusInteractionArea 0))))