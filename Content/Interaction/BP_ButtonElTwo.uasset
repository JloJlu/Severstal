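; Interactable electrical toggle button, apparently part of a puzzle, that highlights through custom depth when focused.
; Interacting while focused plays or reverses a Timeline, based on ElectroON, that slides the mesh slightly along Z.
; When the Timeline finishes, it flips ElectroON and sends ButtonDownMessage to the linked screws, cap, colored arms and final button.
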(event EventInterfaceToggleFocus
  (params (Focus :type Boolean))
  (Rendering|SetRenderCustomDepth (Variables|Default|GetStaticMesh) Focus))

(event EventInteractPick
  (if (stale EventInterfaceToggleFocus Focus)
    (if (Variables|Default|GetElectroON)
      (bind _screw_track (Timeline|Timeline Play)
        (:Update
          (Transformation|SetRelativeLocation (Variables|Default|GetStaticMesh) (Math|Vector|MakeVector 0.0 0.0 (Math|Float|Lerp 0.0 -2.0 _screw_track)) false false))
        (:Finished
          (if (Variables|Default|GetElectroON)
            (Variables|Default|SetElectroON false)
            (else
              (Variables|Default|SetElectroON true)))
          (Utilities|FlowControl|Sequence
            (:then_0
              (Class|BIButton|ButtonDown(Message) (Variables|Default|GetScrew)))
            (:then_1
              (Class|BIButton|ButtonDown(Message) (Variables|Default|GetScrew_0)))
            (:then_2
              (Class|BIButton|ButtonDown(Message) (Variables|Default|GetScrew_1)))
            (:then_3
              (Class|BIButton|ButtonDown(Message) (Variables|Default|GetScrew_2)))
            (:then_4
              (Class|BIButton|ButtonDown(Message) (Variables|Default|GetCap)))
            (:then_5
              (Class|BIButton|ButtonDown(Message) (Variables|Default|GetRedArm)))
            (:then_6
              (Class|BIButton|ButtonDown(Message) (Variables|Default|GetBlueArm)))
            (:then_7
              (Class|BIButton|ButtonDown(Message) (Variables|Default|GetGreenArm)))
            (:then_8
              (Class|BIButton|ButtonDown(Message) (Variables|Default|GetFinalButton))))))
      (else
        (Timeline|Timeline Reverse)))))

(fn ConstructionScript)