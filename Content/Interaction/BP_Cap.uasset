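; BP_Cap is an interactable cover held by four screws that the player can slide open or shut, with a custom-depth highlight on focus.
; Screw events raise or lower a counter, and a focused pick moves the cap only when it reads four and the toggleable electricity flag is off.
; A timeline lerps the mesh position, then flips the open state and messages all four screws.
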(event EventInterfaceToggleFocus
  (params (Focus :type Boolean))
  (Rendering|SetRenderCustomDepth (Variables|Default|GetStaticMesh) Focus))

(event EventOpenCap
  (Variables|Default|SetNumScrew (+ 1.0 (Variables|Default|GetNumScrew))))

(event EventInteractPick
  (if (stale EventInterfaceToggleFocus Focus)
    (if (== 4.0 (Variables|Default|GetNumScrew))
      (if (not (Variables|Default|GetElectroON))
        (if (Variables|Default|GetCapOpen)
          (bind _screw_track (Timeline|Timeline Reverse)
            (:Update
              (Transformation|SetRelativeLocation (Variables|Default|GetStaticMesh) (Math|Vector|MakeVector (Math|Float|Lerp 0.0 -1e+01 _screw_track) 0.0 (Math|Float|Lerp 0.0 -6e+01 _screw_track)) false false))
            (:Finished
              (if (Variables|Default|GetCapOpen)
                (Variables|Default|SetCapOpen false)
                (else
                  (Variables|Default|SetCapOpen true)))
              (Utilities|FlowControl|Sequence
                (:then_0
                  (Class|BIInteractScrewCap|ScrewCap(Message) (Variables|Default|Getscrew)))
                (:then_1
                  (Class|BIInteractScrewCap|ScrewCap(Message) (Variables|Default|Getscrew_1)))
                (:then_2
                  (Class|BIInteractScrewCap|ScrewCap(Message) (Variables|Default|Getscrew_2)))
                (:then_3
                  (Class|BIInteractScrewCap|ScrewCap(Message) (Variables|Default|Getscrew_0))))))
          (else
            (Timeline|Timeline Play)))))))

(event EventButtonDown
  (if (Variables|Default|GetElectroON)
    (Variables|Default|SetElectroON false)
    (else
      (Variables|Default|SetElectroON true))))

(event EventCloseCap
  (Variables|Default|SetNumScrew (+ -1.0 (Variables|Default|GetNumScrew))))

(fn ConstructionScript)