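; Interactable screw that the player removes or refits with a screwdriver, reporting each change to its Cap.
; Focus toggles a custom depth highlight, and interaction requires focus, the screwdriver, power off and the cap closed.
; A timeline spins and slides the mesh out, then hides it and sends the open message; reversing it restores the screw and sends close.
; Pickup, cap and button events update the gating flags.
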(event EventScrewCap
  (if (Variables|Default|GetCapOpen)
    (Variables|Default|SetCapOpen false)
    (else
      (Variables|Default|SetCapOpen true))))

(event EventInterfaceToggleFocus
  (params (Focus :type Boolean))
  (Rendering|SetRenderCustomDepth (Variables|Default|GetStaticMesh) Focus))

(event EventPickUpScrewdriver
  (Variables|Default|SetHasKey true))

(event EventInteractPick
  (bind _staticmesh (Variables|Default|GetStaticMesh))
  (if (stale EventInterfaceToggleFocus Focus)
    (if (Variables|Default|GetHasKey)
      (if (not (Variables|Default|GetElectroOn))
        (if (not (Variables|Default|GetCapOpen))
          (if (Variables|Default|GetVisible)
            (bind _screw_track (Timeline|SCrew%20TimeLine Play)
              (:Update
                (Utilities|FlowControl|Sequence
                  (:then_0
                    (Transformation|SetRelativeRotation _staticmesh (Math|Rotator|MakeRotator (Math|Float|Lerp 0.0 7.2e+02 _screw_track) 0.0 0.0) false false))
                  (:then_1
                    (Transformation|SetRelativeLocation _staticmesh (Math|Vector|MakeVector (Math|Float|Lerp 0.0 -5.0 _screw_track) 0.0 0.0) false false))))
              (:Finished
                (if (Variables|Default|GetVisible)
                  (Class|PrimitiveComponent|SetVisibleinSceneCaptureOnly (Variables|Default|GetStaticMesh) (Variables|Default|GetVisible))
                  (Utilities|FlowControl|Sequence
                    (:then_0
                      (if (Variables|Default|GetVisible)
                        (Variables|Default|SetVisible false)
                        (else
                          (Variables|Default|SetVisible true))))
                    (:then_1
                      (Class|BIInteractCap|OpenCap(Message) (Variables|Default|GetCap))))
                  (else
                    (Utilities|FlowControl|Sequence
                      (:then_0
                        (Class|BIInteractCap|CloseCap(Message) (Variables|Default|GetCap)))
                      (:then_1
                        (if (Variables|Default|GetVisible)
                          (Variables|Default|SetVisible false)
                          (else
                            (Variables|Default|SetVisible true)))))))))
            (else
              (Class|PrimitiveComponent|SetVisibleinSceneCaptureOnly (Variables|Default|GetStaticMesh) (Variables|Default|GetVisible))
              (Timeline|SCrew%20TimeLine Reverse))))))))

(event EventButtonDown
  (if (Variables|Default|GetElectroON)
    (Variables|Default|SetElectroON false)
    (else
      (Variables|Default|SetElectroON true))))

(fn ConstructionScript)