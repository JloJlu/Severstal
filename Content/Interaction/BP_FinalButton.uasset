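; Final button interactable that ends the game by opening the end screen.
; It outlines its mesh on focus; picking it while focused plays a timeline that lowers the mesh slightly.
; When the press finishes, it shows WB_End, pauses the game and enables the mouse cursor.
; Separate events toggle power, colored arm and numbered button flags, which this graph never reads.
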(event EventOne
  (if (Variables|Default|GetButtonOne)
    (Variables|Default|SetButtonOne false)
    (else
      (Variables|Default|SetButtonOne true))))

(event EventThree
  (if (Variables|Default|GetButtonThree)
    (Variables|Default|SetButtonThree false)
    (else
      (Variables|Default|SetButtonThree true))))

(event EventInterfaceToggleFocus
  (params (Focus :type Boolean))
  (Rendering|SetRenderCustomDepth (Variables|Default|GetStaticMesh) Focus))

(event EventRed
  (if (Variables|Default|GetRedArm)
    (Variables|Default|SetRedArm false)
    (else
      (Variables|Default|SetRedArm true))))

(event EventInteractPick
  (if (stale EventInterfaceToggleFocus Focus)
    (bind _screw_track (Timeline|Timeline Play)
      (:Update
        (Transformation|SetRelativeLocation (Variables|Default|GetStaticMesh) (Math|Vector|MakeVector 0.0 0.0 (Math|Float|Lerp 0.0 -2.0 _screw_track)) false false))
      (:Finished
        (bind _returnvalue (UserInterface|CreateWidget "/Game/UI/WB_End.WB_End_C"))
        (UserInterface|Viewport|AddtoViewport _returnvalue 0)
        (Game|SetGamePaused true)
        (Variables|/Script/Engine.PlayerController|SetbShowMouseCursor (Game|GetPlayerController 0) true)
        (Variables|Default|SetPause true)))))

(event EventGreen
  (if (Variables|Default|GetGreenArm)
    (Variables|Default|SetGreenArm false)
    (else
      (Variables|Default|SetGreenArm true))))

(event EventButtonDown
  (if (Variables|Default|GetElectroON)
    (Variables|Default|SetElectroON false)
    (else
      (Variables|Default|SetElectroON true))))

(event EventBlue
  (if (Variables|Default|GetBlueArm)
    (Variables|Default|SetBlueArm false)
    (else
      (Variables|Default|SetBlueArm true))))

(fn ConstructionScript)