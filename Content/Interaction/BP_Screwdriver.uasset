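; BP_Screwdriver is a pickup actor that notifies screws when the screwdriver is picked up.
; The InterfaceToggleFocus event toggles custom depth rendering on the LocationScrewdriver component as focus changes.
; InteractPick checks Focus, then a sequence sends PickUpScrewdriverMessage to four referenced screws, calling DestroyActor right after the first message, ahead of the other three.
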(event EventBeginPlay)

(event Collision|EventActorBeginOverlap
  (params (OtherActor :type Actor%20Object%20Reference)))

(event EventTick
  (params (DeltaSeconds :type Float%20%28single-precision%29)))

(event EventInterfaceToggleFocus
  (params (Focus :type Boolean))
  (Rendering|SetRenderCustomDepth (Variables|Default|GetLocation_Screwdriver) Focus))

(event EventInteractPick
  (if (stale EventInterfaceToggleFocus Focus)
    (Utilities|FlowControl|Sequence
      (:then_0
        (Class|BIScrew|PickUpScrewdriver(Message) (Variables|Default|GetScrew))
        (Actor|DestroyActor))
      (:then_1
        (Class|BIScrew|PickUpScrewdriver(Message) (Variables|Default|GetScrew_0)))
      (:then_2
        (Class|BIScrew|PickUpScrewdriver(Message) (Variables|Default|GetScrew_1)))
      (:then_3
        (Class|BIScrew|PickUpScrewdriver(Message) (Variables|Default|GetScrew_2))))))

(fn ConstructionScript)