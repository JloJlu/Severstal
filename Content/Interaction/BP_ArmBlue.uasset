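; BP_ArmBlue is an interactable blue arm that rotates between two pitch positions and reports to a FinalButton actor.
; Focus toggles custom depth on its mesh for highlighting.
; A pick while focused and with ElectroON off plays or reverses a timeline based on the Arm flag, flipping that flag and sending BlueMessage when finished.
; ButtonDown toggles ElectroON, which blocks interaction while on.
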(event EventInterfaceToggleFocus
  (params (Focus :type Boolean))
  (Rendering|SetRenderCustomDepth (Variables|Default|GetStaticMesh) Focus))

(event EventInteractPick
  (if (stale EventInterfaceToggleFocus Focus)
    (if (not (Variables|Default|GetElectroON))
      (if (Variables|Default|GetArm)
        (bind _screw_track (Timeline|Timeline Play)
          (:Update
            (Transformation|SetRelativeRotation (Variables|Default|GetStaticMesh) (Math|Rotator|MakeRotator 0.0 (Math|Float|Lerp 0.0 9e+01 _screw_track) 0.0) false false))
          (:Finished
            (if (Variables|Default|GetArm)
              (Variables|Default|SetArm false)
              (else
                (Variables|Default|SetArm true)))
            (Class|BIInteractBlue|Blue(Message) (Variables|Default|GetFinalButton))))
        (else
          (Timeline|Timeline Reverse))))))

(event EventButtonDown
  (if (Variables|Default|GetElectroON)
    (Variables|Default|SetElectroON false)
    (else
      (Variables|Default|SetElectroON true))))

(fn ConstructionScript)