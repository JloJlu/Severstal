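; BP_Player is the player-controlled Blueprint that handles movement, look, interaction and UI.
; On BeginPlay it adds the WB_UI widget and the IMC_PlayerInput Enhanced Input context, which drives control-rotation-relative movement and inverted-Y look input.
; F sends InteractPickMessage to overlapping actors that implement BI_InteractPick.
; Hardcoded keys also restart the level (F1) or open WB_Less with the game paused and cursor shown (J).
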(event Input|EnhancedActionEvents|EnhancedInputActionIMC_Move
  (params (ActionValue :type Vector%202D%20Structure) (ElapsedSeconds :type Float%20%28double-precision%29) (TriggeredSeconds :type Float%20%28double-precision%29) (InputAction :type Input%20Action%20Object%20Reference :default "/Game/Input/IMC_Move.IMC_Move"))
  (bind _returnvalue (Pawn|GetControlRotation :!class /Script/Engine.Pawn))
  (bind _returnvalue_2 (Pawn|GetControlRotation :!class /Script/Engine.Pawn))
  (Pawn|Input|AddMovementInput (Math|Vector|GetRightVector (Math|Rotator|MakeRotator (.roll _returnvalue_2) 0.0 (.yaw _returnvalue_2))) (.x ActionValue) false)
  (Pawn|Input|AddMovementInput (Math|Vector|GetForwardVector (Math|Rotator|MakeRotator (.roll _returnvalue) 0.0 (.yaw _returnvalue))) (.y ActionValue) false))

(event Input|EnhancedActionEvents|EnhancedInputActionIMC_Look
  (params (ActionValue :type Vector%202D%20Structure) (ElapsedSeconds :type Float%20%28double-precision%29) (TriggeredSeconds :type Float%20%28double-precision%29) (InputAction :type Input%20Action%20Object%20Reference :default "/Game/Input/IMC_Look.IMC_Look"))
  (Pawn|Input|AddControllerYawInput (.x ActionValue))
  (Pawn|Input|AddControllerPitchInput (* (.y ActionValue) -1.0)))

(event EventBeginPlay
  (Utilities|FlowControl|Sequence
    (:then_0
      (bind _returnvalue (UserInterface|CreateWidget "/Game/UI/WB_UI.WB_UI_C"))
      (UserInterface|Viewport|AddtoViewport _returnvalue 0))
    (:then_1
      (Input|AddMappingContext (PlayerController|LocalPlayerSubsystems|GetEnhancedInputLocalPlayerSubsystem (Game|GetPlayerController 0)) "/Game/Input/IMC_PlayerInput.IMC_PlayerInput" 0 "(bIgnoreAllPressedKeysUntilRelease=True,bForceImmediately=False,bNotifyUserSettings=False)"))))

(event Input|KeyboardEvents|F
  (params (Key :type Key%20Structure :default "None"))
  (:Pressed
    (bind _array_element (Utilities|Array|ForEachLoopwithBreak (Collision|GetOverlappingActors "/Script/Engine.Actor" :!class /Script/Engine.Actor))
      (:LoopBody
        (if (Utilities|DoesObjectImplementInterface _array_element "/Game/Interaction/BI_InteractPick.BI_InteractPick_C")
          (Class|BIInteractPick|InteractPick(Message) _array_element))))))

(event Input|KeyboardEvents|J
  (params (Key :type Key%20Structure :default "None"))
  (:Pressed
    (bind _returnvalue (UserInterface|CreateWidget "/Game/UI/WB_Less.WB_Less_C"))
    (UserInterface|Viewport|AddtoViewport _returnvalue 0)
    (Game|SetGamePaused true)
    (Variables|/Script/Engine.PlayerController|SetbShowMouseCursor (Game|GetPlayerController 0) true)))

(event Input|KeyboardEvents|F1
  (params (Key :type Key%20Structure :default "None"))
  (:Pressed
    (Development|ExecuteConsoleCommand "Restartlevel" 0)))

(fn ConstructionScript)